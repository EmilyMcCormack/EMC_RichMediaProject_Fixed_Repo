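; Suitcase actor that tells the third-person player character when it is inside the suitcase's overlap area.
; BeginPlay caches the player as BP_ThirdPersonCharacter, and overlaps by actors tagged "Player" set that character's InBounds flag true on entry and false on exit.
; Each change sits behind its own DoOnce with no reset wired, so only the first entry and first exit update the flag.
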(event `self.ReceiveBeginPlay`
  (bind _asbp_third_person_character (cast `/Game/ThirdPerson/Blueprints/BP_ThirdPersonCharacter` (`GameplayStatics.GetPlayerCharacter` 0)))
  (set `self.Player` _asbp_third_person_character))

(event `self.ReceiveActorBeginOverlap`
  (params (OtherActor :type "Actor Object Reference"))
  (if (`self.ActorHasTag` OtherActor "Player")
    (`/Engine/EditorBlueprintResources/StandardMacros.DoOnce` false
      (:`Completed`
        (set `/Game/ThirdPerson/Blueprints/BP_ThirdPersonCharacter.InBounds` true (`self.Player`))))))

(event `self.ReceiveActorEndOverlap`
  (params (OtherActor :type "Actor Object Reference"))
  (if (`self.ActorHasTag` OtherActor "Player")
    (`/Engine/EditorBlueprintResources/StandardMacros.DoOnce` false
      (:`Completed`
        (set `/Game/ThirdPerson/Blueprints/BP_ThirdPersonCharacter.InBounds` false (`self.Player`))))))

(fn `UserConstructionScript`)